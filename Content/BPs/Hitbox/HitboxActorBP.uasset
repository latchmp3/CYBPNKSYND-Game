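; Hitbox actor for a two-player fighting game, serving as a proximity, active or hurtbox volume.
; SpawnHitbox colors the display mesh by type, moves it to the hitbox location, shows it and runs a one-off collision check.
; The check finds the opponent via the game mode by comparing its owner to Player1.
; Overlapping that opponent's Hurtbox triggers a proximity reaction or deals damage with stun, blockstun, pushback and launch values.
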(event `SpawnHitbox`
  (switch `EHitboxEnum` (`self.hitboxtype`)
    (:`HB_PROXIMITY`
      (`PrimitiveComponent.SetMaterial` (`self.HitboxDisplay`) 0 "/Game/BPs/Hitbox/Materials/proxHitbox.proxHitbox"))
    (:`HB_ACTIVE`
      (`PrimitiveComponent.SetMaterial` (`self.HitboxDisplay`) 0 "/Game/BPs/Hitbox/Materials/activeHitbox.activeHitbox"))
    (:`HB_HURTBOX`
      (`PrimitiveComponent.SetMaterial` (`self.HitboxDisplay`) 0 "/Game/ODSMannequin/Geometry/Meshes/CubeMaterial.CubeMaterial")))
  (`SceneComponent.K2_SetWorldLocation` (`self.HitboxDisplay`) (`self.hitboxlocation`) false false)
  (`SceneComponent.SetVisibility` (`self.HitboxDisplay`) true false)
  (`self.CheckCollision`))

(event `CheckCollision`
  (bind _player2 (`CyberpunkSyndicatesGameMode.player2` (`self.BaseGameModeReference`)))
  (bind _player1 (`CyberpunkSyndicatesGameMode.player1` (`self.BaseGameModeReference`)))
  (bind _hurtbox (`CyberpunkSyndicatesCharacter.hurtbox` _player1))
  (bind _hurtbox_2 (`CyberpunkSyndicatesCharacter.hurtbox` _player2))
  (bind _isplayerone (`self.DeterminePlayer`))
  (if _isplayerone
    (`/Engine/EditorBlueprintResources/StandardMacros.IsValid` _player2
      (:`Is Valid`
        (`/Engine/EditorBlueprintResources/StandardMacros.IsValid` _hurtbox_2
          (:`Is Valid`
            (if (`self.IsOverlappingActor` _hurtbox_2)
              (switch `EHitboxEnum` (`self.hitboxtype`)
                (:`HB_PROXIMITY`
                  (`CyberpunkSyndicatesCharacter.CollidedWProxHitbox` _player2))
                (:`HB_ACTIVE`
                  (`CyberpunkSyndicatesCharacter.TakeDamage` _player2 (`self.hitboxDamage`) (`self.hitstunTime`) (`self.blockstunTime`) (`self.pushbackDistance`) (`self.launchDistance`)))))))))
    (else
      (`/Engine/EditorBlueprintResources/StandardMacros.IsValid` _player1
        (:`Is Valid`
          (`/Engine/EditorBlueprintResources/StandardMacros.IsValid` _hurtbox
            (:`Is Valid`
              (if (`self.IsOverlappingActor` _hurtbox)
                (switch `EHitboxEnum` (`self.hitboxtype`)
                  (:`HB_PROXIMITY`
                    (`CyberpunkSyndicatesCharacter.CollidedWProxHitbox` _player1))
                  (:`HB_ACTIVE`
                    (`CyberpunkSyndicatesCharacter.TakeDamage` _player1 (`self.hitboxDamage`) (`self.hitstunTime`) (`self.blockstunTime`) (`self.pushbackDistance`) (`self.launchDistance`))))))))))))

(fn `DeterminePlayer`
  (returns (isPlayerOne :type Boolean))
  (bind _ascyberpunk_syndicates_game_mode (cast `CyberpunkSyndicatesGameMode` (`GameplayStatics.GetGameMode`)))
  (bind _output_get (set `self.BaseGameModeReference` _ascyberpunk_syndicates_game_mode))
  (if (== (`CyberpunkSyndicatesGameMode.player1` _output_get) (`self.GetOwner`))
    (return true)
    (else
      (return false))))

(fn `UserConstructionScript`)