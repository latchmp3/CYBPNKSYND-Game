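; Camera actor for a two-player fighting game that frames one character for Blitz and victory shots.
; On BeginPlay, after a short delay, it caches both players from DefaultGameModeBP.
; SwapToBlitzCamera and SwapToVictoryCameraView, currently identical, snap it to an angled view beside the passed character and set the field of view.
; Side offset and yaw mirror with the character's IsFlipped flag, and X is scaled down from the character's position.
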(event `self.ReceiveTick`
  (params (DeltaSeconds :type "Float (single-precision)")))

(event `self.ReceiveBeginPlay`
  (`KismetSystemLibrary.Delay` 0.03)
  (bind _asdefault_game_mode_bp (cast `/Game/BPs/GameMode/DefaultGameModeBP` (`GameplayStatics.GetGameMode`)))
  (bind _player1 (`CyberpunkSyndicatesGameMode.player1` _asdefault_game_mode_bp))
  (`/Engine/EditorBlueprintResources/StandardMacros.IsValid` _player1
    (:`Is Valid`
      (set `self.Player1Ref` _player1)
      (bind _player2 (`CyberpunkSyndicatesGameMode.player2` _asdefault_game_mode_bp))
      (`/Engine/EditorBlueprintResources/StandardMacros.IsValid` _player2
        (:`Is Valid`
          (set `self.Player2Ref` _player2))))))

(event `SwapToBlitzCamera`
  (params (CharacterReference :type "CyberpunkSyndicatesCharacter Object Reference"))
  (bind _returnvalue (`self.GetTransform` (`self.Player1Ref`)))
  (bind _returnvalue_2 (`self.GetTransform` (`self.Player1Ref`)))
  (bind _returnvalue_3 (`self.GetTransform` (`self.Player2Ref`)))
  (bind _returnvalue_4 (`self.GetTransform` (`self.Player2Ref`)))
  (if (== CharacterReference (`self.Player1Ref`))
    (bind _player1ref (`self.Player1Ref`)
      (:`then`
        (if (`CyberpunkSyndicatesCharacter.isFlipped` _player1ref)
          (`self.K2_SetActorTransform` (`KismetMathLibrary.MakeTransform` (`KismetMathLibrary.MakeVector` (/ (.x (.location _returnvalue)) 1.15) (+ (.y (.location _returnvalue)) 155.0) (+ (.z (.location _returnvalue)) 20.0)) (`KismetMathLibrary.MakeRotator` 0.0 0.0 -35.0)))
          (`CameraComponent.SetFieldOfView` (`self.CameraComponent`) 70.0)
          (else
            (`self.K2_SetActorTransform` (`KismetMathLibrary.MakeTransform` (`KismetMathLibrary.MakeVector` (/ (.x (.location _returnvalue_2)) 1.15) (- (.y (.location _returnvalue_2)) 155.0) (+ (.z (.location _returnvalue_2)) 20.0)) (`KismetMathLibrary.MakeRotator` 0.0 0.0 35.0)))
            (`CameraComponent.SetFieldOfView` (`self.CameraComponent`) 70.0))))
      (:`else`))
    (else
      (bind _player2ref (`self.Player2Ref`)
        (:`then`
          (if (`CyberpunkSyndicatesCharacter.isFlipped` _player2ref)
            (`self.K2_SetActorTransform` (`KismetMathLibrary.MakeTransform` (`KismetMathLibrary.MakeVector` (/ (.x (.location _returnvalue_3)) 1.15) (+ (.y (.location _returnvalue_3)) 155.0) (+ (.z (.location _returnvalue_3)) 20.0)) (`KismetMathLibrary.MakeRotator` 0.0 0.0 -35.0)))
            (`CameraComponent.SetFieldOfView` (`self.CameraComponent`) 70.0)
            (else
              (`self.K2_SetActorTransform` (`KismetMathLibrary.MakeTransform` (`KismetMathLibrary.MakeVector` (/ (.x (.location _returnvalue_4)) 1.15) (- (.y (.location _returnvalue_4)) 155.0) (+ (.z (.location _returnvalue_4)) 20.0)) (`KismetMathLibrary.MakeRotator` 0.0 0.0 35.0)))
              (`CameraComponent.SetFieldOfView` (`self.CameraComponent`) 70.0))))
        (:`else`)))))

(event `SwapToVictoryCameraView`
  (params (CharacterReference :type "CyberpunkSyndicatesCharacter Object Reference"))
  (bind _returnvalue (`self.GetTransform` (`self.Player2Ref`)))
  (bind _returnvalue_2 (`self.GetTransform` (`self.Player2Ref`)))
  (bind _returnvalue_3 (`self.GetTransform` (`self.Player1Ref`)))
  (bind _returnvalue_4 (`self.GetTransform` (`self.Player1Ref`)))
  (if (== CharacterReference (`self.Player1Ref`))
    (bind _player1ref (`self.Player1Ref`)
      (:`then`
        (if (`CyberpunkSyndicatesCharacter.isFlipped` _player1ref)
          (`self.K2_SetActorTransform` (`KismetMathLibrary.MakeTransform` (`KismetMathLibrary.MakeVector` (/ (.x (.location _returnvalue_3)) 1.15) (+ (.y (.location _returnvalue_3)) 155.0) (+ (.z (.location _returnvalue_3)) 20.0)) (`KismetMathLibrary.MakeRotator` 0.0 0.0 -35.0)))
          (`CameraComponent.SetFieldOfView` (`self.CameraComponent`) 70.0)
          (else
            (`self.K2_SetActorTransform` (`KismetMathLibrary.MakeTransform` (`KismetMathLibrary.MakeVector` (/ (.x (.location _returnvalue_4)) 1.15) (- (.y (.location _returnvalue_4)) 155.0) (+ (.z (.location _returnvalue_4)) 20.0)) (`KismetMathLibrary.MakeRotator` 0.0 0.0 35.0)))
            (`CameraComponent.SetFieldOfView` (`self.CameraComponent`) 70.0))))
      (:`else`))
    (else
      (bind _player2ref (`self.Player2Ref`)
        (:`then`
          (if (`CyberpunkSyndicatesCharacter.isFlipped` _player2ref)
            (`self.K2_SetActorTransform` (`KismetMathLibrary.MakeTransform` (`KismetMathLibrary.MakeVector` (/ (.x (.location _returnvalue)) 1.15) (+ (.y (.location _returnvalue)) 155.0) (+ (.z (.location _returnvalue)) 20.0)) (`KismetMathLibrary.MakeRotator` 0.0 0.0 -35.0)))
            (`CameraComponent.SetFieldOfView` (`self.CameraComponent`) 70.0)
            (else
              (`self.K2_SetActorTransform` (`KismetMathLibrary.MakeTransform` (`KismetMathLibrary.MakeVector` (/ (.x (.location _returnvalue_2)) 1.15) (- (.y (.location _returnvalue_2)) 155.0) (+ (.z (.location _returnvalue_2)) 20.0)) (`KismetMathLibrary.MakeRotator` 0.0 0.0 35.0)))
              (`CameraComponent.SetFieldOfView` (`self.CameraComponent`) 70.0))))
        (:`else`)))))

(fn `UserConstructionScript`)