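; Game mode for a two-player fighting game, managing player spawning, timed rounds, match wins and rematch resets.
; BeginPlay and rematch share setup that spawns and possesses fighters at tagged PlayerStarts, cross-links them and creates the HUD, with character selection currently yielding TRNDMMYCharacterBP.
; Tick counts down active rounds into TimeOver, which awards the round to the healthier player and ignores ties.
; DetermineMatchWinner compares rounds won against NumRounds.
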(event `ResetMatchValues`
  (bind _player1 (`self.player1`))
  (bind _player2 (`self.player2`))
  ;[1 1 1] Comment
  (set `CyberpunkSyndicatesCharacter.roundsWon` 0 (`self.player1`))
  (set `CyberpunkSyndicatesCharacter.roundsWon` 0 (`self.player2`))
  (bind _foundwidgets (`WidgetBlueprintLibrary.GetAllWidgetsOfClass` "/Game/HUDs/BaseGameModeHUD.BaseGameModeHUD_C"))
  (bind _output (`|GetArrayItem` _foundwidgets))
  (`/Game/HUDs/BaseGameModeHUD.UpdateRoundIndicator` _output 0 0)
  (`/Game/HUDs/BaseGameModeHUD.UpdateRoundIndicator` _output 1 0)
  (`self.K2_DestroyActor` (`self.player1`))
  (`self.K2_DestroyActor` (`self.player2`))
  (set `self.roundTime` 60.0)
  (bind _asbase_game_instance (cast `BaseGameInstance` (`GameplayStatics.GetGameInstance`) :!label _label))
  (bind _output_get (set `self.GameInstanceReference` _asbase_game_instance))
  (set `BaseGameInstance.isDeviceShared` false _output_get)
  (bind _outactors (`GameplayStatics.GetAllActorsOfClass` "/Script/Engine.PlayerStart"))
  (for _array_element _outactors
    (`self.SpawnPlayers` _array_element))
  ;[1 1 1] Set up camera upon rematch
  (bind _outactors_2 (`GameplayStatics.GetAllActorsOfClass` "/Game/BPs/GameMode/FightCameraBP.FightCameraBP_C"))
  (`/Game/BPs/GameMode/FightCameraBP.UseCamera` (`|GetArrayItem` _outactors_2))
  (if (`KismetSystemLibrary.IsValid` (`self.player1`))
    (if (`KismetSystemLibrary.IsValid` (`self.player2`))
      (set `CyberpunkSyndicatesCharacter.otherPlayer` _player2 _player1)
      (set `CyberpunkSyndicatesCharacter.otherPlayer` _player1 _player2)
      (set `CyberpunkSyndicatesCharacter.isFlipped` true _player2)
      (bind _returnvalue (`|CreateWidget` "/Game/HUDs/BaseGameModeHUD.BaseGameModeHUD_C" (`GameplayStatics.GetPlayerController` 0)))
      (`UserWidget.AddToViewport` _returnvalue 0)
      (message `/Game/BPs/GameMode/BasicFunctionInterface.setHUDReferences` (`self.player1`))
      (message `/Game/BPs/GameMode/BasicFunctionInterface.setHUDReferences` (`self.player2`))
      (set `CyberpunkSyndicatesCharacter.isReadyForEntrance` true (`self.player1`)))))

(event `self.ReceiveBeginPlay`
  (goto _label))

(event `RoundStart`
  (set `self.isRoundTimerActive` true)
  (set `CyberpunkSyndicatesCharacter.canAttack` true (`self.player1`))
  (set `CyberpunkSyndicatesCharacter.canAttack` true (`self.player2`))
  (set `CyberpunkSyndicatesCharacter.playerHealth` 1.0 (`self.player1`))
  (set `CyberpunkSyndicatesCharacter.playerHealth` 1.0 (`self.player2`))
  (set `self.roundTime` 60.0))

(event `RoundEnd`
  (set `self.isRoundTimerActive` false)
  (set `CyberpunkSyndicatesCharacter.canAttack` false (`self.player1`))
  (set `CyberpunkSyndicatesCharacter.canAttack` false (`self.player2`)))

(event `self.ReceiveTick`
  (params (DeltaSeconds :type "Float (single-precision)"))
  (bind _returnvalue (- (`self.roundTime`) DeltaSeconds))
  (if (`self.isRoundTimerActive`)
    (if (>= _returnvalue 0.0)
      (set `self.roundTime` _returnvalue)
      (else
        (set `self.roundTime` 0.0)
        (`self.TimeOver`)))))

(fn `DetermineCharacterClass`
  (params (Transform :type "Transform Structure") (Actor :type "Actor Object Reference") (PlayerIndex :type Integer))
  (returns (CharacterReferance :type "/Game/Characters/TRN_DMMY/TRNDMMYCharacterBP Object Reference"))
  (bind _asbase_game_instance (cast `BaseGameInstance` (`GameplayStatics.GetGameInstance`)))
  (switch `int` PlayerIndex
    (:`Default`
      (switch `ECharacterClass` (`BaseGameInstance.P1CharacterClass` _asbase_game_instance) :!label _label
        (:`E_TRNDMMY`
          _)))
    (:`0`
      (goto _label))
    (:`1`
      (switch `ECharacterClass` (`BaseGameInstance.P2CharacterClass` _asbase_game_instance)
        (:`E_TRNDMMY`
          _))))
  (bind _returnvalue (`|SpawnActorFromClass` "/Game/Characters/TRN_DMMY/TRNDMMYCharacterBP.TRNDMMYCharacterBP_C" Transform "Undefined" "OverrideRootScale" Actor null))
  (return _returnvalue))

(fn `DetermineMatchWinner`
  (returns (WinnerIndex :type Integer))
  (if (>= (`CyberpunkSyndicatesCharacter.roundsWon` (`self.player1`)) (`self.numRounds`))
    (`CyberpunkSyndicatesCharacter.WinMatch` (`self.player1`))
    (return 0)
    (elif (>= (`CyberpunkSyndicatesCharacter.roundsWon` (`self.player2`)) (`self.numRounds`))
      (`CyberpunkSyndicatesCharacter.WinMatch` (`self.player2`))
      (return 1)
      (else
        (return -1)))))

(fn `SpawnPlayers`
  (params (Object :type "Actor Object Reference"))
  (bind _returnvalue (`self.GetTransform` Object))
  (bind _asplayer_start (cast `PlayerStart` Object))
  (bind _playerstarttag (`PlayerStart.PlayerStartTag` _asplayer_start))
  (if (== "P1" _playerstarttag)
    (bind _characterreferance (`self.DetermineCharacterClass` (`self.GetTransform` Object) Object))
    (bind _output_get (set `self.player1` _characterreferance))
    (`Controller.Possess` (`GameplayStatics.GetPlayerController` 0) _output_get)
    (elif (== _playerstarttag "P2")
      (bind _characterreferance_2 (`self.DetermineCharacterClass` _returnvalue Object 1))
      (bind _output_get_2 (set `self.player2` _characterreferance_2))
      (if (`BaseGameInstance.isDeviceShared` (`self.GameInstanceReference`))
        (bind _returnvalue_2 (`|SpawnActorFromClass` "/Script/CyberpunkSyndicates.BasePlayerController" _returnvalue "Undefined" "OverrideRootScale" null null))
        (`Controller.Possess` _returnvalue_2 _output_get_2)
        (else
          (bind _outactors (`GameplayStatics.GetAllActorsOfClass` "/Script/Engine.PlayerController"))
          (bind _output (`|GetArrayItem` _outactors 1))
          (`/Engine/EditorBlueprintResources/StandardMacros.IsValid` _output
            (:`Is Valid`
              (`Controller.Possess` _output _output_get_2))))))))

(fn `TimeOver`
  (if (> (`CyberpunkSyndicatesCharacter.playerHealth` (`self.player1`)) (`CyberpunkSyndicatesCharacter.playerHealth` (`self.player2`)))
    (`CyberpunkSyndicatesCharacter.WinRound` (`self.player1`))
    (set `self.roundTime` 60.0)
    (elif (< (`CyberpunkSyndicatesCharacter.playerHealth` (`self.player1`)) (`CyberpunkSyndicatesCharacter.playerHealth` (`self.player2`)))
      (`CyberpunkSyndicatesCharacter.WinRound` (`self.player2`))
      (set `self.roundTime` 60.0))))

(fn `UserConstructionScript`)