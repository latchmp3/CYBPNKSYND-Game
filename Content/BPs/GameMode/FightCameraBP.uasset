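; Fighting-game camera actor that frames both players side-on and can become player 0's view target through UseCamera.
; After a brief startup delay, it reads both players from DefaultGameModeBP, then spawns and positions left and right stage bounds outward from their locations.
; Each tick it tracks the players' Y midpoint and averaged, slightly raised height, offset in X from Player 1, widening FOV with their separation within a clamped range.
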(event `UseCamera`
  (`PlayerController.SetViewTargetWithBlend` (`GameplayStatics.GetPlayerController` 0) self 0.0 "VTBlend_Linear" 0.0 false)
  (`KismetSystemLibrary.Delay` 0.03 :!label _label)
  (bind _asdefault_game_mode_bp (cast `/Game/BPs/GameMode/DefaultGameModeBP` (`GameplayStatics.GetGameMode`)))
  (bind _player1 (`CyberpunkSyndicatesGameMode.player1` _asdefault_game_mode_bp))
  (`/Engine/EditorBlueprintResources/StandardMacros.IsValid` _player1
    (:`Is Valid`
      (set `self.Player1Ref` _player1)
      (bind _player2 (`CyberpunkSyndicatesGameMode.player2` _asdefault_game_mode_bp))
      (`/Engine/EditorBlueprintResources/StandardMacros.IsValid` _player2
        (:`Is Valid`
          (set `self.Player2Ref` _player2)
          (bind _returnvalue (`|SpawnActorFromClass` "/Game/BPs/GameMode/StageBoundsBP.StageBoundsBP_C" (`self.GetTransform`) "Undefined" "OverrideRootScale" null null))
          (set `self.LeftStageBounds` _returnvalue)
          (bind _returnvalue_2 (`|SpawnActorFromClass` "/Game/BPs/GameMode/StageBoundsBP.StageBoundsBP_C" (`self.GetTransform`) "Undefined" "OverrideRootScale" null null))
          (set `self.RightStageBounds` _returnvalue_2)
          (`self.SetCameraBoundaries`))))))

(event `self.ReceiveBeginPlay`
  (goto _label))

(event `self.ReceiveTick`
  (params (DeltaSeconds :type "Float (single-precision)"))
  (bind _player1ref (`self.Player1Ref`))
  (bind _player2ref (`self.Player2Ref`))
  (if (and (`KismetSystemLibrary.IsValid` _player1ref) (`KismetSystemLibrary.IsValid` _player2ref))
    (`self.K2_SetActorLocation` (`KismetMathLibrary.MakeVector` (- (.x (`self.K2_GetActorLocation` (`self.Player1Ref`))) 270.0) (/ (+ (.y (`self.K2_GetActorLocation` _player1ref)) (.y (`self.K2_GetActorLocation` _player2ref))) 2.0) (/ (+ (.z (`self.K2_GetActorLocation` _player1ref)) (.z (`self.K2_GetActorLocation` _player2ref))) 1.9)))
    (`CameraComponent.SetFieldOfView` (`self.CameraComponent`) (`KismetMathLibrary.FClamp` (`KismetMathLibrary.Abs` (* (- (.y (`self.K2_GetActorLocation` (`self.Player1Ref`))) (.y (`self.K2_GetActorLocation` (`self.Player2Ref`)))) 0.225)) 75.0 90.0))))

(fn `SetCameraBoundaries`
  (bind _returnvalue (+ (.y (`self.K2_GetActorLocation` (`self.Player2Ref`))) 1500.0))
  (bind _returnvalue_2 (- (.y (`self.K2_GetActorLocation` (`self.Player1Ref`))) 1500.0))
  (set `self.LeftMax` (- 100.0 _returnvalue_2))
  (`self.K2_SetActorLocation` (`self.LeftStageBounds`) (`KismetMathLibrary.MakeVector` (.x (`self.K2_GetActorLocation` (`self.Player1Ref`))) _returnvalue_2 (.z (`self.K2_GetActorLocation` (`self.Player1Ref`)))) false false)
  (set `self.RightMax` (+ _returnvalue 100.0))
  (`self.K2_SetActorLocation` (`self.RightStageBounds`) (`KismetMathLibrary.MakeVector` (.x (`self.K2_GetActorLocation` (`self.Player2Ref`))) _returnvalue (.z (`self.K2_GetActorLocation` (`self.Player2Ref`)))) false false))

(fn `UserConstructionScript`)