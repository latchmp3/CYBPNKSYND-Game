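; Character Blueprint for TRN_DMMY, a fighter in a two-player fighting game with rounds, rage and entrance sequences.
; On BeginPlay it caches the game mode and Player 2, then spawns and attaches a hurtbox actor.
; Key presses feed a short timestamped input buffer, while separate events build per-player HUD input icon stacks.
; Other events relay round changes, swap the rage material and play side-specific entrances; the damage sound is unwired.
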(event `self.ReceiveBeginPlay`
  (bind _ascyberpunk_syndicates_game_mode (cast `CyberpunkSyndicatesGameMode` (`GameplayStatics.GetGameMode`)))
  (bind _output_get (set `self.GameModeReference` _ascyberpunk_syndicates_game_mode))
  (bind _player2 (`CyberpunkSyndicatesGameMode.player2` _output_get))
  (`/Engine/EditorBlueprintResources/StandardMacros.IsValid` _player2
    (:`Is Valid`
      (set `self.Player2Reference` _player2))
    (:`Is Not Valid`
      _))
  (bind _returnvalue (`|SpawnActorFromClass` "/Game/BPs/Hitbox/HurtboxActorBP.HurtboxActorBP_C" (`self.GetTransform` (`PawnMovementComponent.GetPawnOwner` (`self.CharacterMovement`))) "Undefined" "OverrideRootScale" null null))
  (bind _output_get_2 (set `self.hurtbox` _returnvalue))
  (`self.K2_AttachToActor` _returnvalue self "None" "SnapToTarget" "SnapToTarget" "SnapToTarget" true)
  (`self.K2_AttachToActor` _output_get_2 self "None" "SnapToTarget" "SnapToTarget" "SnapToTarget" true)
  (`self.SetOwner` _returnvalue self))

(event `InputAction|openControlsMenu`
  (params (Key :type "Key Structure"))
  (:`Pressed`
    (bind _returnvalue (`|CreateWidget` "/Game/HUDs/ChangeControlsMenu.ChangeControlsMenu_C"))
    (`UserWidget.AddToViewport` _returnvalue 0)))

(event `self.EnterRage`
  (`PrimitiveComponent.SetMaterial` (`self.Mesh`) 0 "/Game/ODSMannequin/Mannequin/Character/Materials/M_UE4Man_Body_Military.M_UE4Man_Body_Military"))

(event `InputAction|AddToInputBuffer`
  (params (Key :type "Key Structure"))
  (bind _inputbuffer (`self.inputBuffer`))
  (:`Pressed`
    (for _array_element _inputbuffer
      (if (< (`.timeStamp` (break `InputInfo` _array_element)) (- (`GameplayStatics.GetTimeSeconds`) 0.3))
        (`KismetArrayLibrary.Array_RemoveItem` _inputbuffer _array_element)))
    (`self.AddInputToInputBuffer` (make `InputInfo` (`KismetTextLibrary.Conv_TextToString` (`KismetInputLibrary.Key_GetDisplayName` Key)) (`GameplayStatics.GetTimeSeconds`)))))

(event `/Game/BPs/GameMode/BasicFunctionInterface.setHUDReferences`
  (bind _foundwidgets (`WidgetBlueprintLibrary.GetAllWidgetsOfClass` "/Game/HUDs/BaseGameModeHUD.BaseGameModeHUD_C"))
  (set `self.HUDReference` (`|GetArrayItem` _foundwidgets)))

(event `self.AddInputIconToScreen`
  (params (_iconIndex :type Integer) (_shouldAddInput :type Boolean))
  (if _shouldAddInput
    (if (`self.isPlayerOne`)
      (`self.P1AddInputImage` _iconIndex)
      (else
        (`self.P2AddInputImage` _iconIndex)))))

(event `self.PlayDamageSoundEffect`
  ;[1 1 1] sound effects
)

(event `self.NotifyRoundStart`
  (bind _asdefault_game_mode_bp (cast `/Game/BPs/GameMode/DefaultGameModeBP` (`self.GameModeReference`)))
  (`/Game/BPs/GameMode/DefaultGameModeBP.RoundStart` _asdefault_game_mode_bp))

(event `self.NotifyRoundEnd`
  (bind _asdefault_game_mode_bp (cast `/Game/BPs/GameMode/DefaultGameModeBP` (`self.GameModeReference`)))
  (`/Game/BPs/GameMode/DefaultGameModeBP.RoundEnd` _asdefault_game_mode_bp))

(event `self.UpdateHUDRoundIcons`
  (bind _hudreference (`self.HUDReference`)
    (:`then`
      (`/Game/HUDs/BaseGameModeHUD.UpdateRoundIcons` _hudreference))
    (:`else`)))

(fn `P1AddInputImage`
  (params (IconIndex :type Integer))
  (locals (IconImageArray :type "Array of SlateBrush Structure"))
  (bind _p1iconimages (`self.P1IconImages`))
  (bind _returnvalue (`|CreateWidget` "/Game/HUDs/InputStackIcon.InputStackIcon_C"))
  (`KismetArrayLibrary.Array_Insert` (`self.P1IconImages`) _returnvalue)
  (`Image.SetBrush` (`/Game/HUDs/InputStackIcon.InputIcon` _returnvalue) (`|GetArrayItem` (`local.IconImageArray`) IconIndex))
  (bind _hudreference (`self.HUDReference`)
    (:`then`
      (bind _inputstackhorizontalbox (`/Game/HUDs/InputStack.InputStackHorizontalBox` (`/Game/HUDs/BaseGameModeHUD.p1Inputs` _hudreference)))
      (`PanelWidget.ClearChildren` _inputstackhorizontalbox)
      (for _array_element (`self.P1IconImages`)
        (`PanelWidget.AddChild` _inputstackhorizontalbox _array_element)
        (for (_ _array_index) _p1iconimages
          (if (> _array_index 12)
            (`KismetArrayLibrary.Array_Remove` _p1iconimages _array_index)))))
    (:`else`)))

(fn `P2AddInputImage`
  (params (IconIndex :type Integer))
  (locals (IconImageArray :type "Array of SlateBrush Structure"))
  (bind _p2iconimages (`self.P2IconImages`))
  (bind _returnvalue (`|CreateWidget` "/Game/HUDs/InputStackIcon.InputStackIcon_C"))
  (`KismetArrayLibrary.Array_Insert` (`self.P2IconImages`) _returnvalue)
  (`Image.SetBrush` (`/Game/HUDs/InputStackIcon.InputIcon` _returnvalue) (`|GetArrayItem` (`local.IconImageArray`) IconIndex))
  (bind _hudreference (`self.HUDReference`)
    (:`then`
      (bind _inputstackhorizontalbox (`/Game/HUDs/InputStack.InputStackHorizontalBox` (`/Game/HUDs/BaseGameModeHUD.p2inputs` _hudreference)))
      (`PanelWidget.ClearChildren` _inputstackhorizontalbox)
      (for _array_element (`self.P2IconImages`)
        (`PanelWidget.AddChild` _inputstackhorizontalbox _array_element)
        (for (_ _array_index) _p2iconimages
          (if (> _array_index 12)
            (`KismetArrayLibrary.Array_Remove` _p2iconimages _array_index)))))
    (:`else`)))

(fn `PlayEntranceSequence`
  (if (`self.isFlipped`)
    (`PlayerController.SetViewTargetWithBlend` (`GameplayStatics.GetPlayerController` 0) self 0.0 "VTBlend_Linear" 0.0 false)
    (`MovieSceneSequencePlayer.Play` (`ActorSequenceComponent.SequencePlayer` (`self.P1SideEntranceSequence`)))
    (else
      (`PlayerController.SetViewTargetWithBlend` (`GameplayStatics.GetPlayerController` 0) self 0.0 "VTBlend_Linear" 0.0 false)
      (`MovieSceneSequencePlayer.Play` (`ActorSequenceComponent.SequencePlayer` (`self.P2SideEntranceSequence`))))))

(fn `UserConstructionScript`)